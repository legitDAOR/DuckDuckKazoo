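; BP_Hunter is an armed character that shoots at BP_Pato actors and exposes a patrol route.
; BeginPlay caches all patos and their average location once, which Shooting turns toward.
; Shooting, gated by a two-second cooldown, spawns a projectile but damages the first cached pato directly, then signals shooting end.
; WieldGun attaches a pistol to the hand socket, and Tick sets Running from velocity.
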(event Custom|Shooting
  (Transformation|SetActorRotation (Math|Rotator|FindRelativeLookatRotation (Math|Conversions|ToTransform(Vector) (Transformation|GetActorLocation)) (stale EventBeginPlay _returnvalue)))
  (if (Variables|Default|GetbCanAttack?)
    (bind _returnvalue (Game|SpawnActorfromClass "/Game/FirstPerson/Blueprints/BP_FirstPersonProjectile.BP_FirstPersonProjectile_C" (Transformation|GetWorldTransform (Variables|Default|GetShootingLocation)) "Undefined" "MultiplyWithRoot" 0 0))
    (Game|Damage|ApplyDamage (Utilities|Array|Get(acopy) (stale EventBeginPlay _outactors)) 1.0 0 _returnvalue)
    (Variables|Default|SetbCanAttack? false)
    (Utilities|FlowControl|Delay 2.0)
    (Variables|Default|SetbCanAttack? true)
    (Default|CallOnShootingEnd)))

(event Custom|WieldGun
  (bind _returnvalue (Game|SpawnActorfromClass "/Game/DuckDuckKazoo/Hunter/PistolActor/BP_Pistol.BP_Pistol_C" (Transformation|GetActorTransform) "Undefined" "MultiplyWithRoot" 0 0))
  (Transformation|AttachComponentToComponent _returnvalue (Variables|Character|GetMesh) "hand_r_gun_socket" "KeepRelative" "KeepRelative" "KeepRelative" true)
  (Variables|AI|SetbIsWieldingWeapon? true))

(event EventTick
  (params (DeltaSeconds :type Float%20%28single-precision%29))
  (Variables|Default|SetbRunning? (> (Math|Vector|VectorLength (Variables|/Script/Engine.MovementComponent|GetVelocity (Variables|Character|GetCharacterMovement))) 0.0)))

(event EventBeginPlay
  (bind _outactors (Actor|GetAllActorsOfClass "/Game/DuckDuckKazoo/Pato/BP_Pato.BP_Pato_C"))
  (bind _returnvalue (Class|GameplayStatics|GetActorArrayAverageLocation _outactors)))

(fn ConstructionScript)

(fn GetPatrolRoute
  (return (Variables|AI|GetPatrolRoute)))