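; BP_Pato is the player Blueprint in DuckDuckKazoo, handling health and kazoo playing.
; On BeginPlay it creates the WBP_Player widget and fills health, then pushes clamped changes to the widget on damage or when key 2 heals one point.
; Left mouse plays the kazoo sound after a short delay and briefly raises the KazooPlayed flag, with a debug print.
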(event EventBeginPlay
  (bind _maxhealth (Variables|Default|GetMaxHealth))
  (bind _returnvalue (UserInterface|CreateWidget "/Game/DuckDuckKazoo/Pato/PlayerWidgets/WBP_Player.WBP_Player_C"))
  (bind _output_get (Variables|Default|SetWBP_Player _returnvalue))
  (UserInterface|Viewport|AddtoViewport _output_get 0)
  (bind _output_get_2 (Variables|Default|SetCurrentHealth _maxhealth))
  (Default|SetHealth (Variables|Default|GetWBP_Player) _output_get_2 _maxhealth))

(event Game|Damage|EventAnyDamage
  (params (Damage :type Float%20%28single-precision%29) (DamageType :type Damage%20Type%20Object%20Reference) (InstigatedBy :type Controller%20Object%20Reference) (DamageCauser :type Actor%20Object%20Reference))
  ;[0.15 0.15 0.15 0.5] Get Damaged
  (Variables|Default|SetCurrentHealth (Math|Integer|Max(Integer) 0 (- (Variables|Default|GetCurrentHealth) Damage)))
  (Default|SetHealth (Variables|Default|GetWBP_Player) (Variables|Default|GetCurrentHealth) (Variables|Default|GetMaxHealth)))

(event Input|KeyboardEvents|2
  (params (Key :type Key%20Structure :default "None"))
  (bind _maxhealth (Variables|Default|GetMaxHealth))
  ;[0.15 0.15 0.15 0.5] Get Healed
  (:Pressed
    (Variables|Default|SetCurrentHealth (Math|Integer|Min(Integer) _maxhealth (+ 1 (Variables|Default|GetCurrentHealth))))
    (Default|SetHealth (Variables|Default|GetWBP_Player) (Variables|Default|GetCurrentHealth) _maxhealth)))

(event Input|KeyboardEvents|1
  (params (Key :type Key%20Structure :default "None"))
  ;[0.15 0.15 0.15 0.5] Get Damaged
)

(event Input|MouseEvents|LeftMouseButton
  (params (Key :type Key%20Structure :default "None"))
  ;[0.15 0.15 0.15 0.5] Kazoo Played
  (:Pressed
    (Utilities|FlowControl|Delay 0.54)
    (Audio|Components|Audio|Play (Variables|Default|GetKazooSounds) 0.0)
    (Variables|Default|SetbKazooPlayed true)
    (Development|PrintString "Kazoo played" (Variables|Default|GetbKazooPlayed) true "(R=0.000000,G=0.660000,B=1.000000,A=1.000000)" 1.0)
    (Utilities|FlowControl|Delay 0.1)
    (Variables|Default|SetbKazooPlayed false)))

(fn ConstructionScript
  (|CallParentFunction))